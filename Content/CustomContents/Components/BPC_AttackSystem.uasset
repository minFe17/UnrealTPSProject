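; Player attack component handling an unarmed punch combo, rifle fire and rifle aiming from Enhanced Input actions.
; Montage notifies advance the four-hit combo, timers or hit interruptions reset it, and StartAttackTrace schedules a damaging sphere trace at the current hand.
; Rifle fire traces from the camera, then from the muzzle to apply damage.
; Aiming toggles zoom, crosshair and movement-oriented rotation.
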(event Custom|ResetCounter
  ;[0.15 0.15 0.15 0.5] Combo Animation
  (Variables|Default|SetComboCounter 0))

(event Custom|StartAttackTrace
  (bind _returnvalue (Utilities|Time|SetTimerbyEvent (delegate Custom|AttackTrace) 0.01)) ; StartAttackTrace가 실행된 후 0.01 뒤에 AttackTrace  실행
  (Variables|Default|SetAttackTimerHnadler _returnvalue))

(event Custom|AttackTrace
  (bind _playercharacter (Variables|Default|GetPlayerCharacter))
  (bind _playercharacter_2 (Variables|Default|GetPlayerCharacter))
  (bind _lefthand (Variables|/Game/CustomContents/Player/BP_PlayerCharacter.BP_PlayerCharacter_C|GetLefthand _playercharacter_2))
  (bind _righthand (Variables|/Game/CustomContents/Player/BP_PlayerCharacter.BP_PlayerCharacter_C|GetRightHand _playercharacter))
  (bind (_start _end) (CallFunction|GetHandLocation _righthand))
  (bind (_start_2 _end_2) (CallFunction|GetHandLocation _lefthand))
  (switch int (Variables|Default|GetComboCounter)
    (:0
      (CallFunction|AttackSphereTrace _start_2 _end_2 (Variables|Default|GetPlayerCharacter) (Variables|Default|GetBase%20Damage) :!label _label))
    (:1
      (CallFunction|AttackSphereTrace _start _end (Variables|Default|GetPlayerCharacter) (Variables|Default|GetBase%20Damage)))
    (:2
      (goto _label))
    (:3)))

(event Custom|StopAttackTrace
  (Utilities|Time|ClearandInvalidateTimerbyHandle (Variables|Default|GetAttackTimerHnadler)))

(event Custom|ResetByHit
  (if (Variables|/Game/CustomContents/Player/BP_PlayerCharacter.BP_PlayerCharacter_C|GetIsHitting (Variables|Default|GetPlayerCharacter))
    (Variables|Default|SetIsAttacking false)
    (Variables|Default|SetComboCounter 0)))

(event Custom|RifleFire
  (bind _playercharacter (Variables|Default|GetPlayerCharacter))
  (bind _playercharacter_2 (Variables|Default|GetPlayerCharacter))
  (bind _camera (Variables|/Game/CustomContents/Player/BP_PlayerCharacter.BP_PlayerCharacter_C|GetCamera _playercharacter))
  (bind _currentweapon (Variables|/Game/CustomContents/Player/BP_PlayerCharacter.BP_PlayerCharacter_C|GetCurrentWeapon _playercharacter_2))
  (bind _returnvalue (Transformation|GetWorldLocation _camera))
  (bind _returnvalue_2 (Math|Vector|GetForwardVector _camera))
  (bind _weapon (Variables|/Game/CustomContents/Items/Weapons/BP_WeaponMaster.BP_WeaponMaster_C|GetWeapon _currentweapon))
  (bind _returnvalue_3 (Transformation|GetSocketLocation _weapon "Muzzle"))
  (bind _returnvalue_4 (* _returnvalue_2 2e+04))
  (Animation|Montage|PlayMontage (Variables|/Script/Engine.Character|GetMesh (Variables|Default|GetPlayerCharacter)) "/Game/CustomContents/Animations/FireAnimations/MM_Rifle_Fire_Montage.MM_Rifle_Fire_Montage"
    (:then
      (bind (_outhit _returnvalue_5) (Collision|LineTraceByChannel _returnvalue (+ _returnvalue _returnvalue_4) "TraceTypeQuery1" false 0 "ForDuration")) ; 카메라에서 조준
      (if _returnvalue_5
        (bind (_outhit_2 _returnvalue_6) (Collision|LineTraceByChannel _returnvalue_3 (* (Math|Vector|Normalize (- (.ImpactPoint (Collision|BreakHitResult _outhit)) _returnvalue_3)) 2e+04) "TraceTypeQuery1" false 0 "ForDuration"))
        (if _returnvalue_6
          (Game|Damage|ApplyDamage (.HitActor (Collision|BreakHitResult _outhit_2)) 33.0 0 (Variables|Default|GetPlayerCharacter)))
        (else
          (Collision|LineTraceByChannel _returnvalue_3 (+ _returnvalue_3 _returnvalue_4) "TraceTypeQuery1" false 0 "ForDuration"))))))

(event Input|EnhancedActionEvents|EnhancedInputActionIA_Attack
  (params (ActionValue :type Boolean) (ElapsedSeconds :type Float%20%28double-precision%29) (TriggeredSeconds :type Float%20%28double-precision%29) (InputAction :type Input%20Action%20Object%20Reference :default "/Game/CustomContents/Player/Inputs/IA_Attack.IA_Attack"))
  (bind _charactermesh (Variables|Default|GetCharacterMesh))
  ;[0.15 0.15 0.15 0.5] Combo Animation
  (:Started
    (if (Variables|/Game/CustomContents/Player/BP_PlayerCharacter.BP_PlayerCharacter_C|GetIsArmedRifle (Variables|Default|GetPlayerCharacter))
      (CallFunction|RifleFire)
      (elif (and (not (Variables|Default|GetIsAttacking)) (not (Variables|/Game/CustomContents/Player/BP_PlayerCharacter.BP_PlayerCharacter_C|GetIsHitting (Variables|Default|GetPlayerCharacter))))
        (Variables|Default|SetIsAttacking true)
        (switch int (Variables|Default|GetComboCounter)
          (:0
            (Animation|Montage|PlayMontage _charactermesh "/Game/CustomContents/Animations/Montages/Attack1_Jab_Montage.Attack1_Jab_Montage"
              (:then
                (Utilities|Time|SetTimerbyEvent (delegate Custom|ResetCounter) 1.0 :!label _label))
              (:OnInterrupted
                (CallFunction|ResetbyHit))
              (:OnNotifyBegin
                (Variables|Default|SetIsAttacking false)
                (Variables|Default|SetComboCounter 1))))
          (:1
            (Animation|Montage|PlayMontage _charactermesh "/Game/CustomContents/Animations/Montages/Attack2_Straight_Montage.Attack2_Straight_Montage"
              (:then
                (goto _label))
              (:OnInterrupted
                (CallFunction|ResetbyHit))
              (:OnNotifyBegin
                (Variables|Default|SetIsAttacking false)
                (Variables|Default|SetComboCounter 2))))
          (:2
            (Animation|Montage|PlayMontage _charactermesh "/Game/CustomContents/Animations/Montages/Attack3_Hook_Montage.Attack3_Hook_Montage"
              (:then
                (goto _label))
              (:OnInterrupted
                (CallFunction|ResetbyHit))
              (:OnNotifyBegin
                (Variables|Default|SetIsAttacking false)
                (Variables|Default|SetComboCounter 3))))
          (:3
            (Animation|Montage|PlayMontage _charactermesh "/Game/CustomContents/Animations/Montages/Attack4_Hook_Montage.Attack4_Hook_Montage"
              (:then
                (goto _label))
              (:OnInterrupted
                (CallFunction|ResetbyHit))
              (:OnNotifyBegin
                (Variables|Default|SetIsAttacking false)
                (Variables|Default|SetComboCounter 0)))))))))

(event Input|EnhancedActionEvents|EnhancedInputActionIA_Aiming
  (params (ActionValue :type Boolean) (ElapsedSeconds :type Float%20%28double-precision%29) (TriggeredSeconds :type Float%20%28double-precision%29) (InputAction :type Input%20Action%20Object%20Reference :default "/Game/CustomContents/Player/Inputs/IA_Aiming.IA_Aiming"))
  (bind _playercharacter (Variables|Default|GetPlayerCharacter))
  (bind _playercharacter_2 (Variables|Default|GetPlayerCharacter))
  (bind _playercharacter_3 (Variables|Default|GetPlayerCharacter))
  (:Triggered
    (if (Variables|/Game/CustomContents/Player/BP_PlayerCharacter.BP_PlayerCharacter_C|GetIsArmedRifle (Variables|Default|GetPlayerCharacter))
      (Variables|Default|SetIsAiming true)
      (Variables|/Script/Engine.CharacterMovementComponent|SetbOrientRotationToMovement (Variables|/Script/Engine.Character|GetCharacterMovement _playercharacter) false)
      (Variables|/Script/Engine.Pawn|SetbUseControllerRotationYaw _playercharacter true)
      (Default|ZoominbyAiming _playercharacter_3)
      (Widget|SetVisibility (Variables|/Game/CustomContents/UI/WB_HUD.WB_HUD_C|GetCrosshair (Variables|/Game/CustomContents/Player/BP_PlayerController.BP_PlayerController_C|GetPlayerHUD (Variables|/Game/CustomContents/Player/BP_PlayerCharacter.BP_PlayerCharacter_C|GetPlayerController _playercharacter_3))) "Visible")))
  (:Canceled
    (if (Variables|/Game/CustomContents/Player/BP_PlayerCharacter.BP_PlayerCharacter_C|GetIsArmedRifle (Variables|Default|GetPlayerCharacter)) :!label _label
      (Variables|Default|SetIsAiming false)
      (Variables|/Script/Engine.CharacterMovementComponent|SetbOrientRotationToMovement (Variables|/Script/Engine.Character|GetCharacterMovement (Variables|Default|GetPlayerCharacter)) true)
      (Default|ZoomOutbyAiming _playercharacter_2)
      (Widget|SetVisibility (Variables|/Game/CustomContents/UI/WB_HUD.WB_HUD_C|GetCrosshair (Variables|/Game/CustomContents/Player/BP_PlayerController.BP_PlayerController_C|GetPlayerHUD (Variables|/Game/CustomContents/Player/BP_PlayerCharacter.BP_PlayerCharacter_C|GetPlayerController _playercharacter_2))) "Hidden")))
  (:Completed
    (goto _label)))

(event EventBeginPlay
  (bind _asbp_player_character (Utilities|Casting|CastToBP_PlayerCharacter (Components|GetOwner)))
  (bind _output_get (Variables|Default|SetPlayerCharacter _asbp_player_character))
  (Variables|Default|SetCharacterMesh (Variables|/Script/Engine.Character|GetMesh _output_get)))

(fn GetHandLocation
  (params (Hand :type Scene%20Component%20Object%20Reference))
  (return (Transformation|GetWorldLocation Hand) (Math|Transform|TransformLocation (Transformation|GetWorldTransform Hand) (+ (Variables|/Script/Engine.SceneComponent|GetRelativeLocation Hand) (Math|Vector|MakeVector 2e+01 0.0 0.0)))))

(fn AttackSphereTrace
  (params (Start :type Vector) (End :type Vector) (DamageCauser :type Actor%20Object%20Reference) (BaseDamage :type Float%20%28single-precision%29))
  (bind (_outhit _returnvalue) (Collision|SphereTraceByChannel Start End 1e+01 "TraceTypeQuery1" false 0 "ForDuration" true "(R=1.000000,G=0.000000,B=0.000000,A=1.000000)" "(R=0.000000,G=1.000000,B=0.000000,A=1.000000)" 7.0))
  (if _returnvalue
    (Game|Damage|ApplyDamage (.HitActor (Collision|BreakHitResult _outhit)) BaseDamage 0 DamageCauser)))