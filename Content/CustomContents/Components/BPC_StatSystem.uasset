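; Actor component that tracks a character's health and death state and reflects it on the HUD health bar.
; On BeginPlay it finds the first top-level WB_HUD widget and fills health to max.
; Increase and decrease functions take the HUD as a parameter and update the bar before clamping the value.
; DecreaseHealth also sets and returns IsDead once health reaches zero.
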(event EventBeginPlay
  (bind _foundwidgets (Widget|GetAllWidgetsOfClass "/Game/CustomContents/UI/WB_HUD.WB_HUD_C" true))
  (Utilities|IsValid (Utilities|Array|Get(acopy) _foundwidgets)
    (:Is%20Valid
      (CallFunction|InitStat (Utilities|Array|Get(acopy) _foundwidgets)))))

(fn IncreaseHealth
  (params (HealthPoint :type Float%20%28double-precision%29) (PlayerHUD :type WB%20HUD%20Object%20Reference))
  (Variables|Default|SetCurrentHealth (+ HealthPoint (Variables|Default|GetCurrentHealth)))
  (Default|SetHPBarPercent PlayerHUD (Variables|Default|GetCurrentHealth) (Variables|Default|GetMaxHealth))
  (if (>= (Variables|Default|GetCurrentHealth) (Variables|Default|GetMaxHealth))
    (Variables|Default|SetCurrentHealth (Variables|Default|GetMaxHealth))))

(fn DecreaseHealth
  (params (DamagePoint :type Float%20%28double-precision%29) (PlayerHUD :type WB%20HUD%20Object%20Reference))
  (Variables|Default|SetCurrentHealth (- (Variables|Default|GetCurrentHealth) DamagePoint))
  (Default|SetHPBarPercent PlayerHUD (Variables|Default|GetCurrentHealth) (Variables|Default|GetMaxHealth))
  (if (<= (Variables|Default|GetCurrentHealth) 0.0)
    (Variables|Default|SetCurrentHealth 0.0)
    (bind _output_get (Variables|Default|SetIsDead true))
    (return _output_get)
    (else
      (bind _output_get_2 (Variables|Default|SetIsDead false))
      (return _output_get_2))))

(fn InitStat
  (params (PlayerHUD :type WB%20HUD%20Object%20Reference))
  (Variables|Default|SetCurrentHealth (Variables|Default|GetMaxHealth))
  (Default|SetHPBarPercent PlayerHUD (Variables|Default|GetCurrentHealth) (Variables|Default|GetMaxHealth)))