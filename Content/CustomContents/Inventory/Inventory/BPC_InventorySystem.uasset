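; Inventory component that holds a resizable array of item slots and handles stacking and slot swaps between inventories.
; AddItem places units one at a time into a matching stack below its DT_Item StackSize, else the first empty slot.
; When full, it sets IsAddFailed to false, so the loop cannot exit.
; MouseDrop calls ChangeSlot, which swaps differently named items (no merging) and fires OnInventoryUpdated on both inventories.
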(event Custom|MouseDrop
  (params (TargetIndex :type Integer) (BeforeInventorySystem :type BPC%20Inventory%20System%20Object%20Reference) (BeforeIndex :type Integer))
  (CallFunction|ChangeSlot TargetIndex BeforeInventorySystem BeforeIndex))

(event EventBeginPlay
  (Utilities|Array|Resize (Variables|Default|GetSlots) (Variables|Default|GetInventorySize)))

(fn AddItem
  (params (ItemAmount :type Integer) (ItemKey :type Name))
  (LocalVariables|SetAmountLeft ItemAmount)
  (while (and (> (LocalVariables|GetAmountLeft) 0) (not (Variables|Default|GetIsAddFailed)))
    (bind (_arrayindex _foundslot) (CallFunction|FindSlot ItemKey)) ; 인벤토리에서 아이템을 찾는다
    (if _foundslot
      (CallFunction|IncreaseSlotStack _arrayindex 1)
      (Math|Integer|DecrementInt (LocalVariables|GetAmountLeft))
      (elif (.IsSlotAvailable (CallFunction|CheckSlotEmpty))
        (CallFunction|AddtoNewSlot ItemKey 1)
        (Math|Integer|DecrementInt (LocalVariables|GetAmountLeft))
        (else
          (Variables|Default|SetIsAddFailed false))))))

(fn FindSlot
  (params (ItemKey :type Name))
  (for (_array_element _array_index) (Variables|Default|GetSlots)
    (if (== (.ItemName (Utilities|Struct|BreakS_Slot _array_element)) ItemKey)
      (if (< (.Amount (Utilities|Struct|BreakS_Slot _array_element)) (CallFunction|GetStackSize ItemKey))
        (return _array_index true))))
  (return -1 false))

(fn GetStackSize
  (params (ItemKey :type Name))
  (bind _returnvalue (Utilities|GetDataTableRow "/Game/CustomContents/Items/DT_Item.DT_Item" ItemKey)
    (:then
      (return (Utilities|Struct|BreakS_Item _returnvalue)))
    (:RowNotFound
      (return -1))))

(fn IncreaseSlotStack
  (params (Index :type Integer) (Amount :type Integer))
  (bind _slots (Variables|Default|GetSlots))
  (bind _output (Utilities|Array|Get(acopy) _slots Index))
  (bind (_itemname _amount) (Utilities|Struct|BreakS_Slot _output))
  (Utilities|Array|SetArrayElem _slots Index (Utilities|Struct|MakeS_Slot _itemname (+ _amount Amount))))

(fn CheckSlotEmpty
  (for (_array_element _array_index) (Variables|Default|GetSlots)
    (if (== (.Amount (Utilities|Struct|BreakS_Slot _array_element)) 0) ; 슬롯의 아이템 개수가 0인지
      (return true _array_index)))
  (return false -1))

(fn AddtoNewSlot
  (params (ItemKey :type Name) (Amount :type Integer))
  (Utilities|Array|SetArrayElem (Variables|Default|GetSlots) (.EmptySlotIndex (CallFunction|CheckSlotEmpty)) (Utilities|Struct|MakeS_Slot ItemKey Amount)))

(fn ChangeSlot
  (params (TargetIndex :type Integer) (BeforeInventorySystem :type BPC%20Inventory%20System%20Object%20Reference) (BeforeIndex :type Integer))
  (LocalVariables|SetLocalSlot (Utilities|Array|Get(acopy) (Variables|BPC_InventorySystem_C|GetSlots BeforeInventorySystem) BeforeIndex))
  (if (>= TargetIndex 0)
    (if (!= (.ItemName (Utilities|Struct|BreakS_Slot (LocalVariables|GetLocalSlot))) (.ItemName (Utilities|Struct|BreakS_Slot (Utilities|Array|Get(acopy) (Variables|Default|GetSlots) TargetIndex))))
      (Utilities|Array|SetArrayElem (Variables|BPC_InventorySystem_C|GetSlots BeforeInventorySystem) BeforeIndex (Utilities|Array|Get(acopy) (Variables|Default|GetSlots) TargetIndex))
      (Utilities|Array|SetArrayElem (Variables|Default|GetSlots) TargetIndex (LocalVariables|GetLocalSlot))
      (Default|CallOnInventoryUpdated)
      (Default|CallOnInventoryUpdated BeforeInventorySystem))))