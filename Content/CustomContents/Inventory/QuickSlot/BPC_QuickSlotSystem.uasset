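; Quick slot component that stores items assigned from the inventory.
; It sizes its QuickSlots array to QuickSlotSize on BeginPlay.
; A mouse-drop event passes the source inventory component and indices to AddToQuickSlot, which writes that inventory slot's entry into the target quick slot without removing it from the inventory.
; Each assignment then fires OnQuickSlotUpdated to notify listeners.
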(event Custom|MouseDropToQuickSlot
  (params (BPC_InventorySystem :type BPC%20Inventory%20System%20Object%20Reference) (InventoryItemIndex :type Integer) (TargetQuickIndex :type Integer))
  (CallFunction|AddtoQuickSlot BPC_InventorySystem InventoryItemIndex TargetQuickIndex))

(event EventBeginPlay
  (Utilities|Array|Resize (Variables|Default|GetQuickSlots) (Variables|Default|GetQuickSlotSize)))

(fn AddtoQuickSlot
  (params (BPC_InventorySystem :type BPC%20Inventory%20System%20Object%20Reference) (InventoryItemIndex :type Integer) (TargetQuickIndex :type Integer))
  (Utilities|Array|SetArrayElem (Variables|Default|GetQuickSlots) TargetQuickIndex (Utilities|Array|Get(acopy) (Variables|/Game/CustomContents/Inventory/Inventory/BPC_InventorySystem.BPC_InventorySystem_C|GetSlots BPC_InventorySystem) InventoryItemIndex))
  (Default|CallOnQuickSlotUpdated))