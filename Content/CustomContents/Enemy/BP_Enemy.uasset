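; Enemy character Blueprint that hands detected players to its AI controller, performs melee attacks and reacts to damage.
; An overlap detector sets the AI target, while StartAttack and StopAttack control a timer-driven sphere trace along the right arm that damages player-tagged actors.
; Incoming damage feeds the stat component and updates Blackboard hit/death flags, triggering either knockback with a random hit montage or a death montage and delayed destruction.
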(event OnComponentBeginOverlap(TempDetector)
  (params (OverlappedComponent :type Primitive%20Component%20Object%20Reference) (OtherActor :type Actor%20Object%20Reference) (OtherComp :type Primitive%20Component%20Object%20Reference) (OtherBodyIndex :type Integer) (bFromSweep :type Boolean) (SweepResult :type Hit%20Result%20Structure%20%28by%20ref%29))
  (bind _asbp_player_character (Utilities|Casting|CastToBP_PlayerCharacter OtherActor))
  (bind _asaic_enemy (Utilities|Casting|CastToAIC_Enemy (AI|GetAIController self)))
  (Default|SetTarget _asaic_enemy _asbp_player_character))

(event Custom|StartAttack
  (bind _returnvalue (Utilities|Time|SetTimerbyEvent (delegate Custom|Attack) 0.01))
  (Variables|Default|SetAttackTimerHandler _returnvalue))

(event Custom|Attack
  (bind (_outhit _returnvalue) (Collision|SphereTraceByChannel (Transformation|GetWorldLocation (Variables|Default|GetRightArmStart)) (Transformation|GetWorldLocation (Variables|Default|GetRightArmEnd)) 3e+01 "TraceTypeQuery1" false 0 "ForDuration"))
  (if _returnvalue
    (if (Actor|ActorHasTag (.HitActor (Collision|BreakHitResult _outhit)) "Player")
      (Game|Damage|ApplyDamage (.HitActor (Collision|BreakHitResult _outhit)) 2e+01 0 self))))

(event Custom|StopAttack
  (Utilities|Time|ClearandInvalidateTimerbyHandle (Variables|Default|GetAttackTimerHandler)))

(event EventBeginPlay
  (bind _asabp_enemy (Utilities|Casting|CastToABP_Enemy (Components|SkeletalMesh|GetAnimInstance (Variables|Character|GetMesh))))
  (Variables|Default|SetAnimationBP _asabp_enemy))

(event Game|Damage|EventAnyDamage
  (params (Damage :type Float%20%28single-precision%29) (DamageType :type Damage%20Type%20Object%20Reference) (InstigatedBy :type Controller%20Object%20Reference) (DamageCauser :type Actor%20Object%20Reference))
  (bind _output_get (Variables|Default|SetIsHit true))
  (AI|Components|Blackboard|SetValueasBool (AI|GetBlackboard 0) (Variables|Default|GetIsHitBlackboardKey) _output_get)
  (Variables|Default|SetDamage%20Causer DamageCauser)
  (bind _isdead (Default|DecreaseHealth (Variables|Default|GetBPC_StatSystem) Damage))
  (bind _output_get_2 (Variables|Default|SetIs%20Dead _isdead))
  (if _output_get_2
    (AI|Components|Blackboard|SetValueasBool (AI|GetBlackboard 0) (Variables|Default|GetIsDeadBlackboardKey) (Variables|Default|GetIs%20Dead))
    (Animation|PlayAnimMontage "/Game/CustomContents/Animations/Montages/Death_Montage.Death_Montage" 1.0 "None")
    (Collision|SetCollisionEnabled (Variables|Collision|GetCapsuleComponent) "NoCollision")
    (Utilities|FlowControl|Delay 5.0)
    (Actor|DestroyActor)
    (else
      (CallFunction|SetBackEnemyLocation)
      (bind _delaytime (CallFunction|HitAnimation (Variables|Default|GetHitMontages)))
      (Utilities|FlowControl|Delay _delaytime)
      (bind _output_get_3 (Variables|Default|SetIsHit false))
      (AI|Components|Blackboard|SetValueasBool (AI|GetBlackboard 0) (Variables|Default|GetIsHitBlackboardKey) _output_get_3))))

(fn ConstructionScript)

(fn HitAnimation
  (params (Array :type Array%20of%20Anim%20Montage%20Object%20References))
  (bind _returnvalue (Animation|PlayAnimMontage (Utilities|Array|Get(acopy) Array (Math|Random|RandomIntegerinRange 0 (- (Utilities|Array|Length Array) 1))) 1.0 "None"))
  (return _returnvalue))

(fn SetBackEnemyLocation
  (Transformation|SetActorLocation (+ (* (Transformation|GetActorForwardVector (Variables|Default|GetDamage%20Causer)) 2e+01) (Transformation|GetActorLocation)) false false))